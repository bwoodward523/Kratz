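; BP_Item is a cheese pickup that a BP_Rat eats by overlapping it.
; On overlap it calls AddCheese on the rat, plays one of five random chomp sounds, spawns a CheesePoof effect scaled by AddCheese's return value, then destroys itself.
; A SpawnPercentChance helper returns true at a given percent probability but is not called within this Blueprint.
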(event `self.ReceiveActorBeginOverlap`
  (params (OtherActor :type "Actor Object Reference"))
  (bind _returnvalue (`self.K2_GetActorLocation`))
  (set `self.NewVar` (`KismetMathLibrary.RandomIntegerInRange` 0 4))
  (bind _asbp_rat (cast `/Game/Dynamic/BP_Rat` OtherActor))
  (bind _outscore (`/Game/Dynamic/BP_Rat.AddCheese` _asbp_rat))
  (if (== (`self.NewVar`) 0)
    (`GameplayStatics.PlaySoundAtLocation` "/Game/Dynamic/Sounds/ChompSounds/CHAOMP.CHAOMP" _returnvalue (struct) 1.0 1.0 0.0 null null null null)
    (`NiagaraFunctionLibrary.SpawnSystemAtLocation` "/Game/Dynamic/CheesePoof.CheesePoof" _returnvalue (struct) (`KismetMathLibrary.Conv_DoubleToVector` _outscore) :!label _label)
    (`self.K2_DestroyActor`)
    (elif (== (`self.NewVar`) 1)
      (`GameplayStatics.PlaySoundAtLocation` "/Game/Dynamic/Sounds/ChompSounds/CHOMP.CHOMP" _returnvalue (struct) 1.0 1.0 0.0 null null null null)
      (goto _label)
      (elif (== (`self.NewVar`) 2)
        (`GameplayStatics.PlaySoundAtLocation` "/Game/Dynamic/Sounds/ChompSounds/ChompNom.ChompNom" _returnvalue (struct) 1.0 1.0 0.0 null null null null)
        (goto _label)
        (elif (== (`self.NewVar`) 3)
          (`GameplayStatics.PlaySoundAtLocation` "/Game/Dynamic/Sounds/ChompSounds/literalChomp.literalChomp" _returnvalue (struct) 1.0 1.0 0.0 null null null null)
          (goto _label)
          (elif (== (`self.NewVar`) 4)
            (`GameplayStatics.PlaySoundAtLocation` "/Game/Dynamic/Sounds/ChompSounds/nomnomnom.nomnomnom" _returnvalue (struct) 1.0 1.0 0.0 null null null null)
            (goto _label)))))))

(fn `SpawnPercentChance`
  (params (InputPercentSpawnChance :type "Float (double-precision)"))
  (returns (willSpawn :type Boolean))
  (if (< (`KismetMathLibrary.RandomFloatInRange` 0.0 100.0) InputPercentSpawnChance)
    (return true)
    (else
      (return false))))

(fn `UserConstructionScript`)