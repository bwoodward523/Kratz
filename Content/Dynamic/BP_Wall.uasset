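; BP_Wall is a wall actor that kills enemies touching it and fades when a rat approaches.
; Overlaps on the Cube call Death on any BP_AerialEnemy or BP_Rat.
; A second collider, MakeTransparentCOllider, reacts only to BP_Rat by swapping the Cube to a transparent brick material.
; It then creates a dynamic material instance whose OpacityValue is driven by a Timeline, with no logic to restore the original material.
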(event `self.Cube.OnComponentHit`
  (params (HitComponent :type "PrimitiveComponent Object Reference") (OtherActor :type "Actor Object Reference") (OtherComp :type "PrimitiveComponent Object Reference") (NormalImpulse :type "Vector Structure") (Hit :type "HitResult Structure (by ref)")))

(event `self.Cube.OnComponentBeginOverlap`
  (params (OverlappedComponent :type "PrimitiveComponent Object Reference") (OtherActor :type "Actor Object Reference") (OtherComp :type "PrimitiveComponent Object Reference") (OtherBodyIndex :type Integer) (bFromSweep :type Boolean) (SweepResult :type "HitResult Structure (by ref)"))
  (bind _asbp_aerial_enemy (cast `/Game/Dynamic/BP_AerialEnemy` OtherActor)
    (:`then`
      (`/Game/Dynamic/BP_AerialEnemy.Death` _asbp_aerial_enemy))
    (:`CastFailed`
      (bind _asbp_rat (cast `/Game/Dynamic/BP_Rat` OtherActor))
      (`/Game/Dynamic/BP_Rat.Death` _asbp_rat))))

(event `self.MakeTransparentCOllider.OnComponentBeginOverlap`
  (params (OverlappedComponent :type "PrimitiveComponent Object Reference") (OtherActor :type "Actor Object Reference") (OtherComp :type "PrimitiveComponent Object Reference") (OtherBodyIndex :type Integer) (bFromSweep :type Boolean) (SweepResult :type "HitResult Structure (by ref)"))
  (bind _cube (`self.Cube`))
  (cast `/Game/Dynamic/BP_Rat` OtherActor)
  (`PrimitiveComponent.SetMaterial` _cube 0 "/Game/Static/StarterContent/Materials/M_Brick_Clay_OldTransparent.M_Brick_Clay_OldTransparent")
  (bind _returnvalue (`PrimitiveComponent.CreateDynamicMaterialInstance` _cube 0 (`PrimitiveComponent.GetMaterial` _cube 0) "None"))
  (bind _output_get (set `self.TransparentMaterial` _returnvalue))
  (bind (_direction _newtrack_0) (`Timeline|Timeline`)
    (:`Update`
      (`MaterialInstanceDynamic.SetScalarParameterValue` _output_get "OpacityValue" _newtrack_0))))

(fn `UserConstructionScript`)