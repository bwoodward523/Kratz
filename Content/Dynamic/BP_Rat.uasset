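; Player rat character for an endless runner: it runs forward automatically, steers sideways, jumps, dashes and counts collected cheese.
; Tick drives movement, eases the spring arm yaw through flagged 90-degree turns and counter-offsets camera height against the actor's Z.
; Shift/right trigger and W start tick-counted side and impulse dashes with particles; DoForwardDash is never called.
; Death explodes and hides the rat, pins it, then opens levels after a delay.
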(event `self.ReceiveBeginPlay`
  ;[1 1 1] Get On BeginPlay
  (`self.GetInputSystem`)
  (set `self.SavedCameraPosition` (`SceneComponent.RelativeLocation` (`self.Camera`))))

(event `EnhancedInput|/Game/Static/Input/INP_Jump`
  (params (ActionValue :type Boolean) (ElapsedSeconds :type "Float (double-precision)") (TriggeredSeconds :type "Float (double-precision)") (InputAction :type "InputAction Object Reference" :default "/Game/Static/Input/INP_Jump.INP_Jump"))
  (bind _isdead (`self.IsDead`))
  (:`Triggered`
    (if (not _isdead)
      (`self.Jump`)
      (set `self.IsJumping` ActionValue)))
  (:`Completed`
    (if (not _isdead)
      (`self.StopJumping`))))

(event `EnhancedInput|/Game/Static/Input/INP_MoveAround`
  (params (ActionValue :type "Vector2D Structure") (ElapsedSeconds :type "Float (double-precision)") (TriggeredSeconds :type "Float (double-precision)") (InputAction :type "InputAction Object Reference" :default "/Game/Static/Input/INP_MoveAround.INP_MoveAround"))
  (:`Triggered`
    (if (not (`self.IsDead`))
      (`self.AddMovementInput` (`KismetMathLibrary.GetRightVector` (`SpringArmComponent.GetTargetRotation` (`self.SpringArm`))) ActionValue_X))))

(event `self.ReceiveTick`
  (params (DeltaSeconds :type "Float (single-precision)"))
  (bind (_returnvalue_x _returnvalue_y _returnvalue_z) (`KismetMathLibrary.BreakVector` (`self.K2_GetActorLocation`)))
  (bind _tapcountl (`self.TapCountL`))
  (bind _tapcountr (`self.TapCountR`))
  (bind (_savedcameraposition_x _savedcameraposition_y _savedcameraposition_z) (`KismetMathLibrary.BreakVector` (`self.SavedCameraPosition`)))
  (bind _camera (`self.Camera`))
  (bind _camera_2 (`self.Camera`))
  (bind _dusttrail1 (`self.DustTrail1`))
  (bind (_ratinitialposition_location _ratinitialposition_rotation _ratinitialposition_scale) (`KismetMathLibrary.BreakTransform` (`self.RatInitialPosition`)))
  (bind (_relativelocation_x _relativelocation_y) (`KismetMathLibrary.BreakVector` (`SceneComponent.RelativeLocation` _camera_2)))
  (set `self.Delta Seconds` DeltaSeconds)
  (`self.DoTurnLeft`)
  (`self.DoTurnRight`)
  (`SceneComponent.K2_SetRelativeLocation` _camera_2 (`KismetMathLibrary.MakeVector` _relativelocation_x _relativelocation_y (+ _savedcameraposition_z (* _returnvalue_z -1.0))) false false)
  (if (`self.IsDead`)
    (`self.K2_SetActorTransform` (`KismetMathLibrary.MakeTransform` (+ _ratinitialposition_location (0.0 0.0 30.0)) _ratinitialposition_rotation _ratinitialposition_scale) true)
    (set `self.DoOnce` false)
    (else
      (`self.TurnEvent`)
      (if (`SceneComponent.IsVisible` (`self.Mesh`))
        (`self.AddMovementInput` (`KismetMathLibrary.GetForwardVector` (`SpringArmComponent.GetTargetRotation` (`self.SpringArm`))))
        (if (not (`NavMovementComponent.IsFalling` (`self.CharacterMovement`)))
          (`ActorComponent.SetActive` _dusttrail1 true false)
          (else
            (`ActorComponent.SetActive` _dusttrail1 false false)))
        (if (`self.CanSideDash`)
          (if (< _tapcountr 12)
            (`self.DoSideDash` (`KismetMathLibrary.BreakVector2D` (stale `EnhancedInput|/Game/Static/Input/INP_MoveAround` ActionValue)))
            (`/Engine/EditorBlueprintResources/StandardMacros.IncrementInt` _tapcountr
              (:`  `
                (if (< _tapcountl 10) :!label _label
                  (`self.DoForwardDashSexy`)
                  (`/Engine/EditorBlueprintResources/StandardMacros.IncrementInt` _tapcountl)
                  (else
                    (set `self.CanDash` false)
                    (set `self.TapCountL` 0)
                    (set `CharacterMovementComponent.MaxWalkSpeed` 850.0 (`self.CharacterMovement`))))))
            (else
              (set `self.CanSideDash` false)
              (set `self.TapCountR` 0)))
          (elif (`self.CanDash`)
            (goto _label)
            (else
              ;[1 1 1] pan camera back from dash
              (`SceneComponent.K2_SetRelativeLocation` _camera (`KismetMathLibrary.VInterpTo` (`SceneComponent.RelativeLocation` _camera) (0.0 0.0 0.0) (`GameplayStatics.GetWorldDeltaSeconds`) 5.0) true false))))))))

(event `Key|Gamepad_RightTrigger`
  (params (Key :type "Key Structure"))
  (:`Pressed`
    ;[1 1 1] Do Dash
    (set `self.CanSideDash` true :!label _label_2)))

(event `Key|LeftShift`
  (params (Key :type "Key Structure"))
  ;[1 1 1] Do Dash
  (:`Pressed`
    (goto _label_2)))

(event `Key|W`
  (params (Key :type "Key Structure"))
  ;[1 1 1] Do Dash
  (:`Pressed`
    (set `self.CanDash` true)))

(event `Key|A`
  (params (Key :type "Key Structure")))

(event `DoTurnLeft`
  ;[1 1 1] Turning On Trigger
  (if (`self.CanTurnLeft`)
    (set `self.DesiredRot` (`KismetMathLibrary.ComposeRotators` (`self.DesiredRot`) (struct :`Yaw` -90.0)))
    (set `self.TurnState` (+ (`self.TurnState`) -90.0))
    (set `self.CanTurnLeft` false)
    (`KismetSystemLibrary.PrintString` (`KismetStringLibrary.Conv_DoubleToString` (`self.TurnState`)) :!label _label_3)))

(event `DoTurnRight`
  ;[1 1 1] Turning On Trigger
  (if (`self.CanTurnRight`)
    (set `self.DesiredRot` (`KismetMathLibrary.ComposeRotators` (`self.DesiredRot`) (struct :`Yaw` 90.0)))
    (set `self.TurnState` (+ 90.0 (`self.TurnState`)))
    (set `self.CanTurnRight` false)
    (goto _label_3)))

(event `TurnEvent`
  (bind _springarm (`self.SpringArm`))
  (bind _desiredrot (`self.DesiredRot`))
  (bind _returnvalue (`SpringArmComponent.GetTargetRotation` _springarm))
  (bind (_returnvalue_roll _returnvalue_pitch _returnvalue_yaw) (`KismetMathLibrary.BreakRotator` (`KismetMathLibrary.RInterpTo` _returnvalue _desiredrot (`GameplayStatics.GetWorldDeltaSeconds`) 10.0)))
  ;[1 1 1] Turning On Trigger
  (if (!= _returnvalue _desiredrot)
    (`SceneComponent.K2_SetRelativeRotation` _springarm (`KismetMathLibrary.MakeRotator` 0.0 -25.0 _returnvalue_yaw) false false)))

(event `Death`
  (bind _returnvalue (`self.K2_GetActorLocation`))
  ;[1 1 1] Death
  (`self.DisableInput` null)
  (if (`self.DoOnce_0`)
    (set `self.DoOnce_0` false)
    (`GameplayStatics.SpawnEmitterAtLocation` "/Game/Static/StarterContent/Particles/P_Explosion.P_Explosion" _returnvalue (struct) (3.5 3.5 3.5))
    (`GameplayStatics.PlaySoundAtLocation` "/Game/Static/StarterContent/Audio/Explosion01.Explosion01" _returnvalue (struct) 1.0 1.0 0.0 null null null null)
    (`SceneComponent.SetVisibility` (`self.Mesh`) false false)
    (`ActorComponent.SetActive` (`self.DustTrail1`) false false)
    (set `self.IsDead` true)
    (set `self.RatInitialPosition` (`self.GetTransform`))
    (`KismetSystemLibrary.Delay` 1.2)
    (`self.Respawn`)
    (`GameplayStatics.OpenLevel` "EndScreen")))

(event `Respawn`
  ;[1 1 1] Respawn on R
  (`GameplayStatics.OpenLevel` " InfiniteWorld"))

(event `Key|R`
  (params (Key :type "Key Structure"))
  ;[1 1 1] Respawn on R
  (:`Pressed`
    (`self.Respawn`)
    (`KismetSystemLibrary.PrintString` "Hello")))

(fn `AddCheese`
  (`/Engine/EditorBlueprintResources/StandardMacros.IncrementInt` (`self.TotalCheese`)))

(fn `DoForwardDash`
  (params (Scale :type "Float (double-precision)"))
  (locals (NewLocalVar :type "Vector Structure" :default (0.0 0.0 0.0)))
  (bind _returnvalue (`GameplayStatics.GetWorldDeltaSeconds`))
  (bind (_temprotation_roll _temprotation_pitch _temprotation_yaw) (`KismetMathLibrary.BreakRotator` (`self.TempRotation`)))
  (bind _turnstate (`self.TurnState`))
  (bind _superdashforwardspeed (`self.SuperDashForwardSpeed`))
  (bind _newparam (`self.GetSpringArmRotation`))
  (bind _output_get (set `self.Current` (`KismetMathLibrary.VInterpTo` (stale _output_get) (* (`KismetMathLibrary.RotateAngleAxis` (`KismetMathLibrary.GetForwardVector` _newparam) (`self.TurnState`) (0.0 0.0 1.0)) Scale (`self.DashSpeed`) _returnvalue) _returnvalue 100.0)))
  (bind _output_get_2 (set `local.NewLocalVar` _output_get))
  (set `self.TempRotation` (`self.K2_GetActorRotation`))
  (if (!= _turnstate -90.0)
    (`self.K2_SetActorRotation` (`KismetMathLibrary.MakeRotator` 0.0 0.0 _turnstate))
    ;[1 1 1] If TurnState / 90 is Odd
    (if (== (mod (/ (`self.TurnState`) 90.0) 2.0) 1.0)
      (if (< (.x _output_get_2) 0.0)
        (bind _returnvalue_2 (+ (* (.x _output_get_2) -1.0) _superdashforwardspeed))
        (bind _returnvalue_3 (+ (* (.z _output_get_2) -1.0) 0.4))
        (`self.K2_AddActorLocalOffset` (`KismetMathLibrary.MakeVector` _returnvalue_2 (.y _output_get_2) _returnvalue_3) true)
        (else
          (bind _returnvalue_4 (+ (.x _output_get_2) _superdashforwardspeed))
          (bind _returnvalue_5 (+ (.z _output_get_2) 0.4))
          (`self.K2_AddActorLocalOffset` (`KismetMathLibrary.MakeVector` _returnvalue_4 (.y _output_get_2) _returnvalue_5) true)))
      (elif (< (.x _output_get_2) 0.0)
        (`self.K2_AddActorLocalOffset` (`KismetMathLibrary.MakeVector` _returnvalue_2 (.y _output_get_2) _returnvalue_5) true)
        (else
          (`self.K2_AddActorLocalOffset` (`KismetMathLibrary.MakeVector` _returnvalue_4 (.y _output_get_2) _returnvalue_3) true))))
    (else
      (`self.K2_SetActorRotation` (`KismetMathLibrary.MakeRotator` 0.0 0.0 (`self.TurnState`)))
      (if (< (.z _output_get_2) 0.0)
        (`self.K2_AddActorLocalOffset` (`KismetMathLibrary.MakeVector` _returnvalue_4 (.y _output_get_2) _returnvalue_3) true)
        (else
          (`self.K2_AddActorLocalOffset` (`KismetMathLibrary.MakeVector` _returnvalue_2 (.y _output_get_2) _returnvalue_5) true)))))
  (`self.K2_SetActorRotation` (`KismetMathLibrary.MakeRotator` _temprotation_roll _temprotation_pitch (+ _temprotation_yaw (`self.TurnState`))))
  (`NiagaraFunctionLibrary.SpawnSystemAtLocation` "/Game/Dynamic/CheesePoof.CheesePoof" (`self.K2_GetActorLocation`))
  (return))

(fn `DoForwardDashSexy`
  (`CharacterMovementComponent.AddImpulse` (`self.CharacterMovement`) (0.0 0.0 10.0) false)
  (`NiagaraFunctionLibrary.SpawnSystemAtLocation` "/Game/Dynamic/CheesePoof.CheesePoof"))

(fn `DoSideDash`
  (params (Scale :type "Float (double-precision)"))
  (bind _returnvalue (`GameplayStatics.GetWorldDeltaSeconds`))
  (bind _newparam (`self.GetSpringArmRotation`))
  (bind _returnvalue_2 (`KismetMathLibrary.VInterpTo` (stale _output_get) (* (`KismetMathLibrary.GetRightVector` _newparam) Scale (* (`self.SideDashSpeed`) (`self.Delta Seconds`)) _returnvalue) _returnvalue 100.0))
  (bind _output_get (set `self.Current` _returnvalue_2))
  (set `self.TempRotation` (`self.K2_GetActorRotation`))
  (`self.K2_SetActorRotation` (struct))
  (`self.K2_AddActorLocalOffset` _output_get true)
  (`self.K2_AddActorLocalOffset` _returnvalue_2 true)
  (`self.K2_SetActorRotation` (`self.TempRotation`))
  (`NiagaraFunctionLibrary.SpawnSystemAtLocation` "/Game/Dynamic/CheesePoofDash.CheesePoofDash" (`self.K2_GetActorLocation`))
  (return))

(fn `GetInputSystem`
  (bind _returnvalue (pcsubsystem `EnhancedInputLocalPlayerSubsystem` (`GameplayStatics.GetPlayerController` 0)))
  (`/Engine/EditorBlueprintResources/StandardMacros.IsValid` _returnvalue
    (:`Is Valid`
      (`EnhancedInputSubsystemInterface.AddMappingContext` _returnvalue "/Game/Static/Input/IMC_ThirdPerson.IMC_ThirdPerson" 0 (struct)))))

(fn `GetSpringArmRotation`
  (returns (NewParam :type "Rotator Structure"))
  (return (`SpringArmComponent.GetTargetRotation` (`self.SpringArm`))))

(fn `UserConstructionScript`)