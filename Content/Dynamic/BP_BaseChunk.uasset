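; BP_BaseChunk is a sewer level chunk for a rat game, exposing an attach transform.
; Its construction script always spawns a plank, then randomly adds walls and another plank, cheese or spinning spikes with trash and traps, or an aerial enemy, using child actor components.
; When the rat overlaps its trigger, it requests two new chunks and destroys itself after a delay.
; Water kills the rat, and a detection zone launches aerial enemies.
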(event `self.Box.OnComponentBeginOverlap`
  (params (OverlappedComponent :type "PrimitiveComponent Object Reference") (OtherActor :type "Actor Object Reference") (OtherComp :type "PrimitiveComponent Object Reference") (OtherBodyIndex :type Integer) (bFromSweep :type Boolean) (SweepResult :type "HitResult Structure (by ref)"))
  (cast `/Game/Dynamic/BP_Rat` OtherActor)
  (bind _asrat_game_mode (cast `/Game/Dynamic/RatGameMode` (`GameplayStatics.GetGameMode`)))
  (`/Game/Dynamic/RatGameMode.AddSewerChunk` _asrat_game_mode)
  (`/Game/Dynamic/RatGameMode.AddSewerChunk` _asrat_game_mode)
  (`KismetSystemLibrary.Delay` 7.0)
  (`self.K2_DestroyActor`)
  (bind _asrat_game_mode_2 (cast `/Game/Dynamic/RatGameMode` (`GameplayStatics.GetGameMode`)))
  (`/Engine/EditorBlueprintResources/StandardMacros.IncrementInt` (`/Game/Dynamic/RatGameMode.ChunkCount` _asrat_game_mode_2)))

(event `self.Water.OnComponentBeginOverlap`
  (params (OverlappedComponent :type "PrimitiveComponent Object Reference") (OtherActor :type "Actor Object Reference") (OtherComp :type "PrimitiveComponent Object Reference") (OtherBodyIndex :type Integer) (bFromSweep :type Boolean) (SweepResult :type "HitResult Structure (by ref)"))
  (bind _asbp_rat (cast `/Game/Dynamic/BP_Rat` OtherActor))
  (`/Game/Dynamic/BP_Rat.Death` _asbp_rat))

(event `self.ReceiveBeginPlay`
  (bind _returnvalue (`KismetMathLibrary.Normal` (0.0 0.0 0.0)))
  (for _array_element (`self.GetAttachedActors` true true)
    (bind _asplank_0 (cast `/Game/Dynamic/Plank0` _array_element))
    (set `/Game/Dynamic/Plank0.Dir` _returnvalue _asplank_0)
    (`KismetSystemLibrary.PrintString` (`KismetStringLibrary.Conv_VectorToString` _returnvalue))))

(event `self.AerialEnemyDetectionZone.OnComponentBeginOverlap`
  (params (OverlappedComponent :type "PrimitiveComponent Object Reference") (OtherActor :type "Actor Object Reference") (OtherComp :type "PrimitiveComponent Object Reference") (OtherBodyIndex :type Integer) (bFromSweep :type Boolean) (SweepResult :type "HitResult Structure (by ref)"))
  (cast `/Game/Dynamic/BP_Rat` OtherActor)
  (`KismetSystemLibrary.PrintString` "Hello")
  (for _array_element (`self.GetAllChildActors` true)
    (bind _asbp_aerial_enemy (cast `/Game/Dynamic/BP_AerialEnemy` _array_element))
    (`/Game/Dynamic/BP_AerialEnemy.SetDirection` _asbp_aerial_enemy)
    (set `/Game/Dynamic/BP_AerialEnemy.IsMoving` true _asbp_aerial_enemy)))

(fn `GetAttachTransform`
  (returns (NewParam :type "Transform Structure"))
  (return (`SceneComponent.K2_GetComponentToWorld` (`self.AttachPoint`))))

(fn `SetAerialSpawnPoints`
  (set `self.AerialEnemySpawnPoints` (`|MakeArray` (`SceneComponent.GetRelativeTransform` (`self.AerialSpawn`)) (`SceneComponent.GetRelativeTransform` (`self.AerialSpawn1`)) (`SceneComponent.GetRelativeTransform` (`self.AerialSpawn2`)) (`SceneComponent.GetRelativeTransform` (`self.AerialSpawn3`)) (`SceneComponent.GetRelativeTransform` (`self.AerialSpawn4`)))))

(fn `SetTrashSpawnPoints`
  (set `self.TrashSpawnPoints` (`|MakeArray` (`SceneComponent.GetRelativeTransform` (`self.FloatingTrash5`)) (`SceneComponent.GetRelativeTransform` (`self.FloatingTrash4`)) (`SceneComponent.GetRelativeTransform` (`self.FloatingTrash3`)) (`SceneComponent.GetRelativeTransform` (`self.FloatingTrash2`)) (`SceneComponent.GetRelativeTransform` (`self.FloatingTrash1`))))
  (set `self.TrashPointsForDirection` (`|MakeArray` (`SceneComponent.GetRelativeTransform` (`self.Arrow55`)) (`SceneComponent.GetRelativeTransform` (`self.Arrow44`)) (`SceneComponent.GetRelativeTransform` (`self.Arrow33`)) (`SceneComponent.GetRelativeTransform` (`self.Arrow22`)) (`SceneComponent.GetRelativeTransform` (`self.Arrow11`)))))

(fn `SetWallSpawnPoints`
  (set `self.WallSpawnPoints` (`|MakeArray` (`SceneComponent.GetRelativeTransform` (`self.WallSpawnRight`)) (`SceneComponent.GetRelativeTransform` (`self.WallSpawnLeft`)))))

(fn `SpawnAerial`
  (bind _aerialenemyspawnpoints (`self.AerialEnemySpawnPoints`))
  (bind _returnvalue (`AddComponent|NODE_AddChildActorComponent-21` :`RelativeTransform` (`|GetArrayItem` _aerialenemyspawnpoints (`KismetMathLibrary.RandomIntegerInRange` 0 (`KismetArrayLibrary.Array_LastIndex` _aerialenemyspawnpoints)))))
  (return))

(fn `SpawnCheese`
  (bind _cheesespawnarea (`self.CheeseSpawnArea`))
  (bind _cheesespawnarea1 (`self.CheeseSpawnArea1`))
  (bind _returnvalue (`KismetMathLibrary.Conv_VectorToTransform` (`KismetMathLibrary.RandomPointInBoundingBox` (`SceneComponent.RelativeLocation` _cheesespawnarea) (`BoxComponent.GetScaledBoxExtent` _cheesespawnarea))))
  (bind _returnvalue_2 (`KismetMathLibrary.Conv_VectorToTransform` (`KismetMathLibrary.RandomPointInBoundingBox` (`SceneComponent.RelativeLocation` _cheesespawnarea1) (`BoxComponent.GetScaledBoxExtent` _cheesespawnarea1))))
  (for _index (range 11)
    (if (>= _index 5)
      (`AddComponent|NODE_AddChildActorComponent-5` :`RelativeTransform` (`KismetMathLibrary.MakeTransform` (`KismetMathLibrary.MakeVector` (.x (.location _returnvalue)) (.y (.location _returnvalue)) 30.0) (.rotation _returnvalue) (.scale _returnvalue)))
      (else
        (`AddComponent|NODE_AddChildActorComponent-9` :`RelativeTransform` (`KismetMathLibrary.MakeTransform` (`KismetMathLibrary.MakeVector` (.x (.location _returnvalue_2)) (.y (.location _returnvalue_2)) 30.0) (.rotation _returnvalue_2) (.scale _returnvalue_2)))))))

(fn `SpawnPlank`
  (returns (PlankDirection :type "Vector Structure"))
  (bind _trashspawnpoints (`self.TrashSpawnPoints`))
  (bind _returnvalue (`KismetMathLibrary.RandomIntegerInRange` 0 (`KismetArrayLibrary.Array_LastIndex` _trashspawnpoints)))
  (bind _output (`|GetArrayItem` _trashspawnpoints _returnvalue))
  (bind _output_location (`KismetMathLibrary.BreakTransform` (`|GetArrayItem` _trashspawnpoints _returnvalue)))
  (bind _output_location_2 (`KismetMathLibrary.BreakTransform` (`|GetArrayItem` (`self.TrashPointsForDirection`) _returnvalue)))
  (set `self.Index` _returnvalue)
  (if (< (`KismetMathLibrary.RandomIntegerInRange` 0 10) 11)
    (`AddComponent|NODE_AddChildActorComponent-12` :`RelativeTransform` (`KismetMathLibrary.MakeTransform` (`KismetMathLibrary.MakeVector` (.x (.location _output)) (.y (.location _output)) (- (.z (.location _output)) 25.0)) (.rotation _output) (.scale _output)))
    (return (- _output_location _output_location_2))))

(fn `SpawnRatTrap`
  (bind _returnvalue_location (`KismetMathLibrary.BreakTransform` (`SceneComponent.GetRelativeTransform` (`self.ArrowTrap1`))))
  (bind _returnvalue_location_2 (`KismetMathLibrary.BreakTransform` (`SceneComponent.GetRelativeTransform` (`self.ArrowTrap`))))
  (if (< (`KismetMathLibrary.RandomIntegerInRange` 0 100) 80)
    (if (== (`KismetMathLibrary.RandomIntegerInRange` 0 1) 0)
      (`AddComponent|NODE_AddChildActorComponent-17` :`RelativeTransform` (`KismetMathLibrary.MakeTransform` _returnvalue_location_2))
      (else
        (`AddComponent|NODE_AddChildActorComponent-18` :`RelativeTransform` (`KismetMathLibrary.MakeTransform` _returnvalue_location))))))

(fn `SpawnSpinningSpike`
  (bind _returnvalue_location (`KismetMathLibrary.BreakTransform` (`SceneComponent.GetRelativeTransform` (`self.ArrowSpike`))))
  (`AddComponent|NODE_AddChildActorComponent-13` :`RelativeTransform` (`KismetMathLibrary.MakeTransform` _returnvalue_location (struct) (2.0 2.0 2.0)))
  (if (<= (`KismetMathLibrary.RandomIntegerInRange` 0 10) 1)
    (`AddComponent|NODE_AddChildActorComponent-14` :`RelativeTransform` (`KismetMathLibrary.MakeTransform` _returnvalue_location (struct :`Yaw` 180.0) (2.0 2.0 2.0)))))

(fn `SpawnTrash`
  (bind _returnvalue (`KismetMathLibrary.RandomIntegerInRange` 0 4))
  (bind _returnvalue_2 (`KismetMathLibrary.RandomIntegerInRange` 0))
  (bind _trashspawnpoints (`self.TrashSpawnPoints`))
  (bind _output (`|GetArrayItem` (`self.TrashSpawnPoints`) _returnvalue_2))
  (bind _returnvalue_3 (`KismetMathLibrary.RandomIntegerInRange` 0 (`KismetArrayLibrary.Array_LastIndex` _trashspawnpoints)))
  (bind _output_2 (`|GetArrayItem` _trashspawnpoints _returnvalue_3))
  (if (< _returnvalue 5)
    (`AddComponent|NODE_AddChildActorComponent-6` :`RelativeTransform` (`KismetMathLibrary.MakeTransform` (`KismetMathLibrary.MakeVector` (.x (.location _output_2)) (.y (.location _output_2)) 40.0) (struct :`Pitch` 180.0) (.scale _output_2)))
    ;[1 1 1] Prob of spawning another trash actor (5/10)
    (if (< _returnvalue 2)
      (while (== _returnvalue_2 _returnvalue_3)
        (set `self.Rand` 0))
      (`AddComponent|NODE_AddChildActorComponent-7` :`RelativeTransform` (`KismetMathLibrary.MakeTransform` (`KismetMathLibrary.MakeVector` (.x (.location _output)) (.y (.location _output)) -100.0) (struct :`Pitch` 90.0) (.scale _output))))))

(fn `SpawnWalls`
  (bind _returnvalue (`KismetMathLibrary.RandomIntegerInRange` 0 10))
  (bind _returnvalue_2 (`KismetMathLibrary.RandomIntegerInRange` 0))
  (bind _wallspawnpoints (`self.WallSpawnPoints`))
  (bind _returnvalue_3 (`KismetMathLibrary.RandomIntegerInRange` 0 (`KismetArrayLibrary.Array_LastIndex` _wallspawnpoints)))
  (if (< _returnvalue 11)
    (`AddComponent|NODE_AddChildActorComponent-1` :`RelativeTransform` (`|GetArrayItem` _wallspawnpoints _returnvalue_3))
    ;[1 1 1] Prob of spawning another wall (5/10)
    (if (< _returnvalue 5)
      (while (== _returnvalue_2 _returnvalue_3)
        _)
      (`AddComponent|NODE_AddChildActorComponent-2` :`RelativeTransform` (`|GetArrayItem` (`self.WallSpawnPoints`) _returnvalue_2)))))

(fn `UserConstructionScript`
  (locals (NewLocalVar :type Integer :default 0) (LocalChunkCount :type Integer :default 0) (Selector :type Integer))
  (bind _asrat_game_mode (cast `/Game/Dynamic/RatGameMode` (`GameplayStatics.GetGameMode`)))
  (set `local.LocalChunkCount` (`/Game/Dynamic/RatGameMode.ChunkCount` _asrat_game_mode))
  (`self.SetWallSpawnPoints`)
  (`self.SetAerialSpawnPoints`)
  (`self.SetTrashSpawnPoints`)
  (`self.SpawnPlank`)
  (switch `int` (`KismetMathLibrary.RandomIntegerInRange` 0 3)
    (:`Default`
      (`self.SpawnWalls` :!label _label)
      (bind _plankdirection (`self.SpawnPlank`))
      (set `self.Plank Direction` _plankdirection))
    (:`0`
      (goto _label))
    (:`1`
      (`self.SpawnCheese`)
      (`self.SpawnTrash`)
      (`self.SpawnRatTrap`))
    (:`2`
      (`self.SpawnSpinningSpike`)
      (`self.SpawnTrash`)
      (`self.SpawnRatTrap`))
    (:`3`
      (`self.SpawnAerial`))))