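; BP_AerialEnemy is a flying kamikaze enemy that targets BP_Rat and explodes on impact.
; While not moving, it faces the rat and bobs on a sine wave.
; When IsMoving is true, Tick sweeps it along a direction toward the rat, re-aimed only while Timer stays below 0.4.
; Hitting the rat kills both, walls kill only the enemy, and an experimental prediction event is not called here.
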(event `SetLookAt`
  (bind (_returnvalue_roll _returnvalue_pitch _returnvalue_yaw) (`KismetMathLibrary.BreakRotator` (`KismetMathLibrary.FindLookAtRotation` (`self.K2_GetActorLocation` (stale `self.ReceiveBeginPlay` _returnvalue)) (`self.K2_GetActorLocation`))))
  (set `self.LookAtPlayer` (`KismetMathLibrary.MakeRotator` _returnvalue_roll _returnvalue_pitch (+ _returnvalue_yaw -90.0))))

(event `SetDirectionPredict`
  (bind _returnvalue (`self.K2_GetActorLocation`))
  ;[1 1 1] Attempting at predicting movement direction
  (bind _returnvalue_2 (`GameplayStatics.GetActorOfClass` "/Game/Dynamic/BP_Rat.BP_Rat_C"))
  (bind _output_get (set `self.Dir` (`KismetMathLibrary.Normal` (- (`self.K2_GetActorLocation` _returnvalue_2) _returnvalue))))
  (set `self.PredictionDir` (+ _output_get (`KismetMathLibrary.Cross_VectorVector` _output_get _returnvalue)))
  (set `self.RandomRot` 0.0))

(event `self.ReceiveBeginPlay`
  (bind _returnvalue (`GameplayStatics.GetActorOfClass` "/Game/Dynamic/BP_Rat.BP_Rat_C"))
  (bind _returnvalue_2 (`GameplayStatics.GetActorOfClass` "/Game/Dynamic/BP_Rat.BP_Rat_C" :!label _label))
  (bind _returnvalue_3 (`self.K2_GetActorLocation` _returnvalue_2))
  (set `self.Dir` (`KismetMathLibrary.Normal` (- (+ _returnvalue_3 (* _returnvalue_3 0.01)) (`self.K2_GetActorLocation`)))))

(event `SetDirection`
  (goto _label))

(event `self.ReceiveTick`
  (params (DeltaSeconds :type "Float (single-precision)"))
  (bind _timer (`self.Timer`))
  (bind _returnvalue (+ _timer (* _timer (`self.Delta Seconds`))))
  (bind _returnvalue_2 (+ (* (`self.Dir`) (* (`self.Delta Seconds`) (`self.Speed`))) (`self.K2_GetActorLocation`)))
  (set `self.Delta Seconds` DeltaSeconds)
  (if (`self.IsMoving`)
    ;[1 1 1] Update Location and face player
    (`AddComponent|NODE_AddRandomVector-0` :`RelativeTransform` (`KismetMathLibrary.Conv_VectorToTransform` _returnvalue_2))
    (bind (_returnvalue_roll _returnvalue_pitch _returnvalue_yaw) (`KismetMathLibrary.BreakRotator` (`KismetMathLibrary.FindLookAtRotation` (`self.K2_GetActorLocation`) (`self.K2_GetActorLocation` (stale `self.ReceiveBeginPlay` _returnvalue)))))
    (`self.K2_SetActorLocationAndRotation` _returnvalue_2 (`KismetMathLibrary.MakeRotator` _returnvalue_roll _returnvalue_pitch (+ _returnvalue_yaw 90.0)) true)
    (if (< (stale _output_get) 0.4)
      (`self.SetDirection`)
      (bind _output_get (set `self.Timer` _returnvalue))
      (`KismetSystemLibrary.PrintString` (`KismetStringLibrary.Conv_DoubleToString` _returnvalue)))
    (else
      (`self.SetLookAt`)
      (`self.K2_SetActorRotation` (`self.LookAtPlayer`))
      (bind _output_get_2 (set `self.PrevZHoverAdd` (`KismetMathLibrary.FInterpEaseInOut` (* (`KismetMathLibrary.Sin` (* (`self.GetGameTimeSinceCreation`) 5.0)) 1.0) (stale _output_get_2) 0.0 10.0)))
      (`SceneComponent.K2_AddRelativeLocation` (`self.DefaultSceneRoot`) (`KismetMathLibrary.MakeVector` 0.0 0.0 _output_get_2) false false))))

(event `self.ReceiveHit`
  (params (MyComp :type "PrimitiveComponent Object Reference") (Other :type "Actor Object Reference") (OtherComp :type "PrimitiveComponent Object Reference") (bSelfMoved :type Boolean) (HitLocation :type "Vector Structure") (HitNormal :type "Vector Structure") (NormalImpulse :type "Vector Structure") (Hit :type "HitResult Structure (by ref)"))
  (bind _asbp_rat (cast `/Game/Dynamic/BP_Rat` Other)
    (:`then`
      (`self.Death`)
      (`/Game/Dynamic/BP_Rat.Death` _asbp_rat))
    (:`CastFailed`
      (cast `/Game/Dynamic/BP_Wall` Other)
      (`self.Death`))))

(event `self.Enemy.OnComponentBeginOverlap`
  (params (OverlappedComponent :type "PrimitiveComponent Object Reference") (OtherActor :type "Actor Object Reference") (OtherComp :type "PrimitiveComponent Object Reference") (OtherBodyIndex :type Integer) (bFromSweep :type Boolean) (SweepResult :type "HitResult Structure (by ref)")))

(event `Death`
  (`GameplayStatics.SpawnEmitterAtLocation` "/Game/Static/StarterContent/Particles/P_Explosion.P_Explosion" (`self.K2_GetActorLocation`))
  (`GameplayStatics.PlaySoundAtLocation` "/Game/Static/StarterContent/Audio/Explosion01.Explosion01" (0.0 0.0 0.0) (struct) 1.0 1.0 0.0 null null null null)
  (`self.K2_DestroyActor`))

(fn `UserConstructionScript`)