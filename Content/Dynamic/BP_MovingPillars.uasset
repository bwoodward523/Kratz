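; BP_MovingPillars is a rotating obstacle that kills the rat character when its Cube is hit by it.
; On BeginPlay its RotatingMovement gets a random single-axis speed, followed by a coin-flip branch that does nothing.
; Tick also adds a fixed, frame-rate-dependent local rotation on top of that movement.
; Cube hits cast the other actor to BP_Rat and call Death.
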(event `self.Cube.OnComponentHit`
  (params (HitComponent :type "PrimitiveComponent Object Reference") (OtherActor :type "Actor Object Reference") (OtherComp :type "PrimitiveComponent Object Reference") (NormalImpulse :type "Vector Structure") (Hit :type "HitResult Structure (by ref)"))
  (bind _asbp_rat (cast `/Game/Dynamic/BP_Rat` OtherActor))
  (`/Game/Dynamic/BP_Rat.Death` _asbp_rat))

(event `self.ReceiveBeginPlay`
  (set `RotatingMovementComponent.RotationRate` (`KismetMathLibrary.MakeRotator` 0.0 0.0 (`KismetMathLibrary.RandomFloatInRange` 40.0 100.0)) (`self.RotatingMovement`))
  (if (== (`KismetMathLibrary.RandomIntegerInRange` 0 1) 0)
    _))

(event `self.ReceiveTick`
  (params (DeltaSeconds :type "Float (single-precision)"))
  (`self.K2_AddActorLocalRotation` (struct :`Yaw` 1.0)))

(fn `UserConstructionScript`)