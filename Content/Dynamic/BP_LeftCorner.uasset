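; Left-corner sewer chunk for an endless rat runner, exposing an attach transform for chaining.
; Its construction script randomly populates it with either walls at preset points or cheese scattered across two box areas; trash spawning is stubbed out.
; A trigger box asks RatGameMode to add a chunk, then destroys this one after a delay.
; The turn zone enables the rat's left turn, while water overlaps and obstacle hits kill it.
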(event `self.Box.OnComponentBeginOverlap`
  (params (OverlappedComponent :type "PrimitiveComponent Object Reference") (OtherActor :type "Actor Object Reference") (OtherComp :type "PrimitiveComponent Object Reference") (OtherBodyIndex :type Integer) (bFromSweep :type Boolean) (SweepResult :type "HitResult Structure (by ref)"))
  (cast `/Game/Dynamic/BP_Rat` OtherActor)
  (bind _asrat_game_mode (cast `/Game/Dynamic/RatGameMode` (`GameplayStatics.GetGameMode`)))
  (`/Game/Dynamic/RatGameMode.AddSewerChunk` _asrat_game_mode)
  (`KismetSystemLibrary.Delay` 10.0)
  (`self.K2_DestroyActor`))

(event `self.TurnZone.OnComponentBeginOverlap`
  (params (OverlappedComponent :type "PrimitiveComponent Object Reference") (OtherActor :type "Actor Object Reference") (OtherComp :type "PrimitiveComponent Object Reference") (OtherBodyIndex :type Integer) (bFromSweep :type Boolean) (SweepResult :type "HitResult Structure (by ref)"))
  (bind _asbp_rat (cast `/Game/Dynamic/BP_Rat` OtherActor))
  (set `/Game/Dynamic/BP_Rat.CanTurnLeft` true _asbp_rat))

(event `self.Water2.OnComponentBeginOverlap`
  (params (OverlappedComponent :type "PrimitiveComponent Object Reference") (OtherActor :type "Actor Object Reference") (OtherComp :type "PrimitiveComponent Object Reference") (OtherBodyIndex :type Integer) (bFromSweep :type Boolean) (SweepResult :type "HitResult Structure (by ref)"))
  (bind _asbp_rat (cast `/Game/Dynamic/BP_Rat` OtherActor))
  (`/Game/Dynamic/BP_Rat.Death` _asbp_rat))

(event `self.Water.OnComponentBeginOverlap`
  (params (OverlappedComponent :type "PrimitiveComponent Object Reference") (OtherActor :type "Actor Object Reference") (OtherComp :type "PrimitiveComponent Object Reference") (OtherBodyIndex :type Integer) (bFromSweep :type Boolean) (SweepResult :type "HitResult Structure (by ref)"))
  (bind _asbp_rat (cast `/Game/Dynamic/BP_Rat` OtherActor))
  (`/Game/Dynamic/BP_Rat.Death` _asbp_rat))

(event `self.Shape_Cube.OnComponentHit`
  (params (HitComponent :type "PrimitiveComponent Object Reference") (OtherActor :type "Actor Object Reference") (OtherComp :type "PrimitiveComponent Object Reference") (NormalImpulse :type "Vector Structure") (Hit :type "HitResult Structure (by ref)"))
  (bind _asbp_rat (cast `/Game/Dynamic/BP_Rat` OtherActor))
  (`/Game/Dynamic/BP_Rat.Death` _asbp_rat))

(event `self.Shape_Cube1.OnComponentHit`
  (params (HitComponent :type "PrimitiveComponent Object Reference") (OtherActor :type "Actor Object Reference") (OtherComp :type "PrimitiveComponent Object Reference") (NormalImpulse :type "Vector Structure") (Hit :type "HitResult Structure (by ref)"))
  (bind _asbp_rat (cast `/Game/Dynamic/BP_Rat` OtherActor))
  (`/Game/Dynamic/BP_Rat.Death` _asbp_rat))

(event `self.Shape_Cube5.OnComponentHit`
  (params (HitComponent :type "PrimitiveComponent Object Reference") (OtherActor :type "Actor Object Reference") (OtherComp :type "PrimitiveComponent Object Reference") (NormalImpulse :type "Vector Structure") (Hit :type "HitResult Structure (by ref)"))
  (bind _asbp_rat (cast `/Game/Dynamic/BP_Rat` OtherActor))
  (`/Game/Dynamic/BP_Rat.Death` _asbp_rat))

(event `self.Shape_Cube7.OnComponentHit`
  (params (HitComponent :type "PrimitiveComponent Object Reference") (OtherActor :type "Actor Object Reference") (OtherComp :type "PrimitiveComponent Object Reference") (NormalImpulse :type "Vector Structure") (Hit :type "HitResult Structure (by ref)"))
  (bind _asbp_rat (cast `/Game/Dynamic/BP_Rat` OtherActor))
  (`/Game/Dynamic/BP_Rat.Death` _asbp_rat))

(event `self.StaticMesh7.OnComponentHit`
  (params (HitComponent :type "PrimitiveComponent Object Reference") (OtherActor :type "Actor Object Reference") (OtherComp :type "PrimitiveComponent Object Reference") (NormalImpulse :type "Vector Structure") (Hit :type "HitResult Structure (by ref)"))
  (bind _asbp_rat (cast `/Game/Dynamic/BP_Rat` OtherActor))
  (`/Game/Dynamic/BP_Rat.Death` _asbp_rat))

(event `self.Shape_Cube8.OnComponentHit`
  (params (HitComponent :type "PrimitiveComponent Object Reference") (OtherActor :type "Actor Object Reference") (OtherComp :type "PrimitiveComponent Object Reference") (NormalImpulse :type "Vector Structure") (Hit :type "HitResult Structure (by ref)"))
  (bind _asbp_rat (cast `/Game/Dynamic/BP_Rat` OtherActor))
  (`/Game/Dynamic/BP_Rat.Death` _asbp_rat))

(fn `GetAttachTransform`
  (returns (NewParam :type "Transform Structure"))
  (return (`SceneComponent.K2_GetComponentToWorld` (`self.AttachPoint`))))

(fn `SetTrashSpawnPoints`
  (set `self.TrashSpawnPoints` (`|MakeArray` (`SceneComponent.GetRelativeTransform` (`self.FloatingTrash5`)) (`SceneComponent.GetRelativeTransform` (`self.FloatingTrash4`)) (`SceneComponent.GetRelativeTransform` (`self.FloatingTrash3`)) (`SceneComponent.GetRelativeTransform` (`self.FloatingTrash2`)) (`SceneComponent.GetRelativeTransform` (`self.FloatingTrash1`)))))

(fn `SetWallSpawnPoints`
  (set `self.WallSpawnPoints` (`|MakeArray` (`SceneComponent.GetRelativeTransform` (`self.WallSpawnRight`)) (`SceneComponent.GetRelativeTransform` (`self.WallSpawnLeft`)))))

(fn `SpawnCheese`
  (bind _cheesespawnarea (`self.CheeseSpawnArea`))
  (bind _cheesespawnarea1 (`self.CheeseSpawnArea1`))
  (bind _returnvalue (`KismetMathLibrary.Conv_VectorToTransform` (`KismetMathLibrary.RandomPointInBoundingBox` (`SceneComponent.RelativeLocation` _cheesespawnarea) (`BoxComponent.GetScaledBoxExtent` _cheesespawnarea))))
  (bind _returnvalue_2 (`KismetMathLibrary.Conv_VectorToTransform` (`KismetMathLibrary.RandomPointInBoundingBox` (`SceneComponent.RelativeLocation` _cheesespawnarea1) (`BoxComponent.GetScaledBoxExtent` _cheesespawnarea1))))
  (for _index (range 11)
    (if (>= _index 5)
      (`AddComponent|NODE_AddChildActorComponent-5` :`RelativeTransform` (`KismetMathLibrary.MakeTransform` (`KismetMathLibrary.MakeVector` (.x (.location _returnvalue)) (.y (.location _returnvalue)) 30.0) (.rotation _returnvalue) (.scale _returnvalue)))
      (else
        (`AddComponent|NODE_AddChildActorComponent-9` :`RelativeTransform` (`KismetMathLibrary.MakeTransform` (`KismetMathLibrary.MakeVector` (.x (.location _returnvalue_2)) (.y (.location _returnvalue_2)) 30.0) (.rotation _returnvalue_2) (.scale _returnvalue_2)))))))

(fn `SpawnTrash`)

(fn `SpawnWalls`
  (bind _returnvalue (`KismetMathLibrary.RandomIntegerInRange` 0 10))
  (bind _returnvalue_2 (`KismetMathLibrary.RandomIntegerInRange` 0))
  (bind _wallspawnpoints (`self.WallSpawnPoints`))
  (bind _returnvalue_3 (`KismetMathLibrary.RandomIntegerInRange` 0 (`KismetArrayLibrary.Array_LastIndex` _wallspawnpoints)))
  (if (< _returnvalue 8)
    (`AddComponent|NODE_AddChildActorComponent-1` :`RelativeTransform` (`|GetArrayItem` _wallspawnpoints _returnvalue_3))
    ;[1 1 1] Prob of spawning another wall (5/10)
    (if (< _returnvalue 5)
      (while (== _returnvalue_2 _returnvalue_3)
        _)
      (`AddComponent|NODE_AddChildActorComponent-2` :`RelativeTransform` (`|GetArrayItem` (`self.WallSpawnPoints`) _returnvalue_2)))))

(fn `UserConstructionScript`
  (`self.SetWallSpawnPoints`)
  (switch `int` (`KismetMathLibrary.RandomIntegerInRange` 0 1)
    (:`0`
      (`self.SpawnWalls`)
      (`self.SpawnTrash`))
    (:`1`
      (`self.SpawnCheese`)
      (`self.SpawnTrash`))))