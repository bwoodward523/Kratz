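; BP_Trap is a trap actor that kills rats on physical contact.
; Hit events on its Trap, Trap1, Trap2 and StaticMesh components each cast the other actor to BP_Rat and call its Death function.
; Other actors are ignored, and the construction script, BeginPlay and Tick add no behavior.
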(event `self.Trap.OnComponentHit`
  (params (HitComponent :type "PrimitiveComponent Object Reference") (OtherActor :type "Actor Object Reference") (OtherComp :type "PrimitiveComponent Object Reference") (NormalImpulse :type "Vector Structure") (Hit :type "HitResult Structure (by ref)"))
  (bind _asbp_rat (cast `/Game/Dynamic/BP_Rat` OtherActor))
  (`/Game/Dynamic/BP_Rat.Death` _asbp_rat))

(event `self.Trap1.OnComponentHit`
  (params (HitComponent :type "PrimitiveComponent Object Reference") (OtherActor :type "Actor Object Reference") (OtherComp :type "PrimitiveComponent Object Reference") (NormalImpulse :type "Vector Structure") (Hit :type "HitResult Structure (by ref)"))
  (bind _asbp_rat (cast `/Game/Dynamic/BP_Rat` OtherActor))
  (`/Game/Dynamic/BP_Rat.Death` _asbp_rat))

(event `self.StaticMesh.OnComponentHit`
  (params (HitComponent :type "PrimitiveComponent Object Reference") (OtherActor :type "Actor Object Reference") (OtherComp :type "PrimitiveComponent Object Reference") (NormalImpulse :type "Vector Structure") (Hit :type "HitResult Structure (by ref)"))
  (bind _asbp_rat (cast `/Game/Dynamic/BP_Rat` OtherActor))
  (`/Game/Dynamic/BP_Rat.Death` _asbp_rat))

(event `self.Trap2.OnComponentHit`
  (params (HitComponent :type "PrimitiveComponent Object Reference") (OtherActor :type "Actor Object Reference") (OtherComp :type "PrimitiveComponent Object Reference") (NormalImpulse :type "Vector Structure") (Hit :type "HitResult Structure (by ref)"))
  (bind _asbp_rat (cast `/Game/Dynamic/BP_Rat` OtherActor))
  (`/Game/Dynamic/BP_Rat.Death` _asbp_rat))

(fn `UserConstructionScript`)